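; AIC_Boar is the AI controller for boar enemies.
; On possession it casts the pawn to BP_Boar, runs BT_Boar, hands the blackboard to the boar and turns on its patrol flag.
; AI perception events are forwarded straight to the boar pawn, which handles the responses itself.
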(event `self.ReceiveBeginPlay`
  (`parent.ReceiveBeginPlay`))

(event `self.ReceivePossess`
  (params (PossessedPawn :type "Pawn Object Reference"))
  (bind _as_bp_boar (`self.As BP Boar`))
  (`parent.ReceivePossess` PossessedPawn)
  (bind _asbp_boar (cast `/Game/Blueprints/Enemies/BP_Boar` PossessedPawn))
  (set `self.As BP Boar` _asbp_boar)
  (`self.RunBehaviorTree` "/Game/Blueprints/Enemies/BT_Boar.BT_Boar")
  (set `/Game/Blueprints/Enemies/BaseEnemy/BP_Character_BaseEnemy.BlackBoard` (`AIBlueprintHelperLibrary.GetBlackboard` null) _as_bp_boar)
  (`/Game/Blueprints/Enemies/BaseEnemy/BP_Character_BaseEnemy.Set_BB_Bool` _as_bp_boar "Patrol?" true))

(event `self.AIPerception.OnTargetPerceptionUpdated`
  (params (Actor :type "Actor Object Reference") (Stimulus :type "AIStimulus Structure"))
  (`/Game/Blueprints/Enemies/BP_Boar.TargetPerceptionUpdate` (`self.As BP Boar`) Actor Stimulus))

(event `self.AIPerception.OnPerceptionUpdated`
  (params (UpdatedActors :type "Array of Actor Object Reference (by ref)"))
  (`/Game/Blueprints/Enemies/BP_Boar.PerceptionUpdate` (`self.As BP Boar`) UpdatedActors))

(fn `UserConstructionScript`
  (`parent.UserConstructionScript`))