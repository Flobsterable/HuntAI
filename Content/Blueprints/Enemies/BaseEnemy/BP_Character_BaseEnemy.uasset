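; Base enemy character with stubbed attack and death, plus patrol, eating and sleep behaviors meant to drive an AI Blackboard.
; On possession it spawns a patrol TargetPoint, and GetPointToMove returns random reachable points nearby or the food target's location.
; Perception events store seen actors, which Eating searches for more BP_Food until satiety is full.
; State changes call SetBBBool, but its Blackboard write is disconnected, so keys never update.
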(event `self.ReceivePossessed`
  (params (NewController :type "Controller Object Reference"))
  ;[1 1 1] Spawn PatrolTargetPoint after Possessed
  (bind _returnvalue (`|SpawnActorFromClass` "/Script/Engine.TargetPoint" (`KismetMathLibrary.MakeTransform` (`self.K2_GetActorLocation` self)) "Undefined" "OverrideRootScale" null null))
  (`KismetArrayLibrary.Array_Add` (`self.PatrolTargetPoints`) _returnvalue)
  (bind _output_get (set `self.Patrol?` true))
  (`self.Set_BB_Bool` "Patrol?" _output_get))

(event `Attack`
  (`KismetSystemLibrary.PrintString` "Attack"))

(event `Death`
  (`KismetSystemLibrary.PrintString` "Death"))

(event `TargetPerceptionUpdate`
  (params (Actor :type "Actor Object Reference") (Stimulus :type "AIStimulus Structure"))
  (set `self.SeenActor` Actor)
  (set `self.AIStimulus` Stimulus))

(event `PerceptionUpdate`
  (params (UpdatedActors :type "Array of Actor Object Reference"))
  (set `self.SeenActors` UpdatedActors))

(fn `ChoosingAttack`
  (returns (NewParam :type Boolean))
  (return false))

(fn `Eating`
  (params (Target :type "/Game/Blueprints/BP_Food Object Reference"))
  (bind _returnvalue (+ (`/Game/Blueprints/BP_Food.SatietyPoints` Target) (`self.CurrentSatiety`)))
  (if (< _returnvalue (`self.Satiety`))
    (set `self.CurrentSatiety` _returnvalue)
    (`self.K2_DestroyActor`)
    (for _array_element (`self.SeenActors`)
      (bind (_asbp_food _bsuccess) (cast `/Game/Blueprints/BP_Food` _array_element :!pure true))
      (if _bsuccess
        (set `self.TargetActor` _asbp_food)
        (`self.Set_BB_Bool` "SeeFood?" true)
        (break)))
    (else
      (set `self.CurrentSatiety` (`self.Satiety`))
      (bind _output_get (set `self.Hungry?` false))
      (`self.Set_BB_Bool` "Hungry?" _output_get)
      (`self.Set_BB_Bool` "SeeFood?")
      (`self.K2_DestroyActor`))))

(fn `GetPointToMove`
  (params (TypeAction :type "/Game/Blueprints/Enemies/E_TypeAction Enum" :default "NewEnumerator0"))
  (returns (TargetLocation :type "Vector Structure"))
  (bind _patroltargetpoints (`self.PatrolTargetPoints`))
  (switch `/Game/Blueprints/Enemies/E_TypeAction` TypeAction
    (:`NewEnumerator0`
      (if (`KismetArrayLibrary.Array_IsValidIndex` _patroltargetpoints)
        (return (`NavigationSystemV1.K2_GetRandomReachablePointInRadius` (`self.K2_GetActorLocation` (`KismetArrayLibrary.Array_Random` _patroltargetpoints)) (`self.PatrolTargetRadius`) null null))
        (else
          (return (`NavigationSystemV1.K2_GetRandomReachablePointInRadius` (`self.K2_GetActorLocation` self) (`self.PatrolTargetRadius`) null null)))))
    (:`NewEnumerator2`
      (return (`self.K2_GetActorLocation` (`self.TargetActor`))))))

(fn `Set_BB_Bool`
  (params (KeyName :type Name) (BoolValue :type Boolean)))

(fn `Sleep`
  (bind _output_get (set `self.Tired?` false))
  (`self.Set_BB_Bool` "Tired?" _output_get)
  (bind _output_get_2 (set `self.Patrol?` true))
  (`self.Set_BB_Bool` "Patrol?" _output_get_2))

(fn `UserConstructionScript`)