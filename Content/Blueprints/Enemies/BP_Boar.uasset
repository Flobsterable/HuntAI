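; Boar enemy Blueprint whose AI patrols, tires, spots food and shelters, and can charge a seen enemy.
; On possession it enables patrol and, after a short delay, sets the blackboard Tired flag.
; Perception updates flag sensed food on the blackboard and collect concealment actors as shelters.
; Charge capsule-traces toward the seen enemy and moves to its location only if the hit actor is a base enemy character.
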(event `self.ReceivePossessed`
  (params (NewController :type "Controller Object Reference"))
  (`parent.ReceivePossessed` NewController)
  (set `self.Patrol?` true)
  (`KismetSystemLibrary.Delay` 5.0)
  (`self.Set_BB_Bool` "Tired?" true))

(event `Charge`
  (bind _outhit (`KismetSystemLibrary.CapsuleTraceSingle` (`self.K2_GetActorLocation` self) (`self.K2_GetActorLocation` (`self.SeenEnemy`)) 20.0 0.0 "TraceTypeQuery1"))
  (if (`.bSuccess` (cast `/Game/Blueprints/Enemies/BaseEnemy/BP_Character_BaseEnemy` (`.HitActor` (`GameplayStatics.BreakHitResult` _outhit)) :!pure true))
    (`|AIMoveTo` null (`self.K2_GetActorLocation` (`self.SeenEnemy`)) null)))

(event `TargetPerceptionUpdate`
  (params (Actor :type "Actor Object Reference") (Stimulus :type "AIStimulus Structure"))
  (bind (_asbp_food _bsuccess) (cast `/Game/Blueprints/BP_Food` (`self.SeenActor`) :!pure true))
  (bind (_asbp_concealment_actor _bsuccess_2) (cast `/Game/Blueprints/BP_ConcealmentActor` (`self.SeenActor`) :!pure true))
  (set `self.SeenActor` Actor)
  (set `self.AIStimulus` Stimulus)
  (if (`.bSuccessfullySensed` (break `AIStimulus` Stimulus))
    (if _bsuccess
      (set `self.SeenFood` _asbp_food)
      (`self.Set_BB_Bool` "SeeFood?" true)
      (elif _bsuccess_2
        (`KismetArrayLibrary.Array_Add` (`self.Shelters`) _asbp_concealment_actor)))))

(event `PerceptionUpdate`
  (params (UpdatedActors :type "Array of Actor Object Reference")))

(fn `UserConstructionScript`
  (`parent.UserConstructionScript`))